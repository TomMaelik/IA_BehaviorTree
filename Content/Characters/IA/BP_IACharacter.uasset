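; BP_IACharacter is an AI-controlled character that detects the third-person player through AI Perception.
; On BeginPlay it runs the BTT_BrainIA behavior tree and caches its Blackboard.
; Sensing the player sets PlayerREF and IsinAlert; losing them clears PlayerREF and stores LastSeenLocation, leaving IsinAlert set.
; A random-point wander loop using AIMoveTo remains in the graph, unconnected and never executed.
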(event OnTargetPerceptionUpdated(AIPerception)
  (params (Actor :type Actor%20Object%20Reference) (Stimulus :type AI%20Stimulus%20Structure))
  (bind _returnvalue (Utilities|Name|MakeLiteralName "PlayerREF"))
  (bind _asbp_third_person_character (Utilities|Casting|CastToBP_ThirdPersonCharacter Actor))
  (if (.bsuccessfullysensed Stimulus)
    (AI|Components|Blackboard|SetValueasObject (Variables|Default|GetBLackBoardREF) _returnvalue _asbp_third_person_character)
    (AI|Components|Blackboard|SetValueasBool (Variables|Default|GetBLackBoardREF) (Utilities|Name|MakeLiteralName "IsinAlert") true)
    (else
      (AI|Components|Blackboard|ClearValue (Variables|Default|GetBLackBoardREF) _returnvalue)
      (AI|Components|Blackboard|SetValueasVector (Variables|Default|GetBLackBoardREF) (Utilities|Name|MakeLiteralName "LastSeenLocation") (.stimuluslocation Stimulus)))))

(event EventBeginPlay
  (bind _returnvalue (Pawn|GetController))
  ;[0 0 0 0.5] Control
  (bind _asaicontroller (Utilities|Casting|CastToAIController _returnvalue))
  (AI|RunBehaviorTree _asaicontroller "/Game/Characters/IA/BTT_BrainIA.BTT_BrainIA")
  (Variables|Default|SetBLackBoardREF (AI|GetBlackboard _returnvalue)))

(fn ConstructionScript)