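; NPC character Blueprint that runs the BT_NPC behavior tree on its AI controller at BeginPlay.
; Perception updates for the player character write it to the PlayerREF blackboard key and cancel the LostVision timer.
; A two-second timer is meant to clear that key, but the branch condition is constant true, so it never starts.
; An older random-point wandering loop using AIMoveTo remains disconnected.
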(event OnTargetPerceptionUpdated(AIPerception)
  (params (Actor :type Actor%20Object%20Reference) (Stimulus :type AI%20Stimulus%20Structure))
  (bind _asbp_third_person_character (Utilities|Casting|CastToBP_ThirdPersonCharacter Actor))
  (if true
    (AI|Components|Blackboard|SetValueasObject (AI|GetBlackboard (Pawn|GetController)) (Utilities|Name|MakeLiteralName "PlayerREF") _asbp_third_person_character)
    (Utilities|Time|ClearandInvalidateTimerbyHandle (Variables|Default|GetLostVision))
    (else
      (bind _returnvalue (Utilities|Time|SetTimerbyEvent (delegate Custom|CustomEvent) 2.0))
      (Variables|Default|SetLostVision _returnvalue))))

(event Custom|CustomEvent
  (AI|Components|Blackboard|ClearValue (AI|GetBlackboard (Pawn|GetController)) (Utilities|Name|MakeLiteralName "PlayerREF")))

(event EventBeginPlay
  ;[0 0 0 0.5] Control
  (bind _asaicontroller (Utilities|Casting|CastToAIController (Pawn|GetController)))
  (AI|RunBehaviorTree _asaicontroller "/Game/Characters/NPC/BT_NPC.BT_NPC"))

(fn ConstructionScript)