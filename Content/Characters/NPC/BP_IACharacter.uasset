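; BP_IACharacter is an NPC character that runs the BTT_BrainIA behavior tree and uses AI perception to track the player.
; When it senses BP_ThirdPersonCharacter, it stores the reference in the blackboard and cancels any pending lost-vision timer.
; Losing the stimulus starts a short timer that clears the player reference and records the stimulus location as last seen.
; An older random-roam movement loop remains but is unconnected.
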(event OnTargetPerceptionUpdated(AIPerception)
  (params (Actor :type Actor%20Object%20Reference) (Stimulus :type AI%20Stimulus%20Structure))
  (bind _asbp_third_person_character (Utilities|Casting|CastToBP_ThirdPersonCharacter Actor))
  (if (.bsuccessfullysensed Stimulus)
    (AI|Components|Blackboard|SetValueasObject (AI|GetBlackboard (Pawn|GetController)) (Utilities|Name|MakeLiteralName "PlayerREF") _asbp_third_person_character)
    (Utilities|Time|ClearandInvalidateTimerbyHandle (Variables|Default|GetLostVision))
    (else
      (bind _returnvalue (Utilities|Time|SetTimerbyEvent (delegate Custom|CustomEvent) 2.0))
      (Variables|Default|SetLostVision _returnvalue))))

(event Custom|CustomEvent
  (bind _returnvalue (Pawn|GetController))
  (bind _returnvalue_2 (AI|GetBlackboard _returnvalue))
  (AI|Components|Blackboard|ClearValue _returnvalue_2 (Utilities|Name|MakeLiteralName "PlayerREF"))
  (AI|Components|Blackboard|SetValueasVector _returnvalue_2 (Utilities|Name|MakeLiteralName "LastSeenLoc") (.stimuluslocation (stale OnTargetPerceptionUpdated(AIPerception) Stimulus))))

(event EventBeginPlay
  ;[0 0 0 0.5] Control
  (bind _asaicontroller (Utilities|Casting|CastToAIController (Pawn|GetController)))
  (AI|RunBehaviorTree _asaicontroller "/Game/Characters/NPC/BTT_BrainIA.BTT_BrainIA"))

(fn ConstructionScript)